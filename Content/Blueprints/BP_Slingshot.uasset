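; BP_Slingshot is a pinball slingshot that kicks the ball away and awards points when the ball overlaps it.
; On overlap with a BP_Ball, it adds score through BP_PinballGameMode and applies an impulse along the capsule's reversed forward vector.
; The SlingBounce timeline animates the bounce by driving the PercentOut parameter on a dynamic material instance created in the construction script.
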(event `self.ReceiveActorBeginOverlap`
  (params (OtherActor :type "Actor Object Reference"))
  (bind _asbp_ball (cast `/Game/Blueprints/BP_Ball` OtherActor))
  (bind _asbp_pinball_game_mode (cast `/Game/Blueprints/BP_PinballGameMode` (`GameplayStatics.GetGameMode`))
    (:`then`
      (`/Game/Blueprints/BP_PinballGameMode.AddScore` _asbp_pinball_game_mode 20.0))
    (:`CastFailed`
      _))
  (`PrimitiveComponent.AddImpulse` (`/Game/Blueprints/BP_Ball.Ball` _asbp_ball) (* (`SceneComponent.GetForwardVector` (`self.Capsule`)) -2500.0) "None" false)
  (bind (_direction _bounce) (`Timeline|SlingBounce` :!via `PlayFromStart`)
    (:`Update`
      (bind _asmaterial_instance_dynamic (cast `MaterialInstanceDynamic` (`PrimitiveComponent.GetMaterial` (`self.StaticMesh`) 2)))
      (`MaterialInstanceDynamic.SetScalarParameterValue` _asmaterial_instance_dynamic "PercentOut" _bounce))))

(fn `UserConstructionScript`
  (`PrimitiveComponent.CreateDynamicMaterialInstance` (`self.StaticMesh`) 2 null))